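; BP_LootComponent is a base loot component that defines how an item behaves when taken.
; Take either calls Use immediately when UseAfterTake is set, or passes the component to TakeItem on player 0's BP_PlayerStateNight, returning the result either way.
; Use is a stub that returns false, and the event graph holds no active logic.
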(fn `take`
  (returns (Taked :type Boolean))
  (if (`self.UseAfterTake`)
    (bind _used (`self.use`))
    (return _used)
    (else
      (bind _asbp_player_state_night (cast `/Game/GameNight/Blueprints/Player/BP_PlayerStateNight` (`GameplayStatics.GetPlayerState` 0)))
      (bind _taked (`/Game/GameNight/Blueprints/Player/BP_PlayerStateNight.TakeItem` _asbp_player_state_night self))
      (return _taked))))

(fn `use`
  (returns (Used :type Boolean))
  (return false))